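; BP_BlackHole_Test is a test black hole actor that pulls in nearby components and destroys static mesh actors at its core.
; Every Tick, components overlapping the outer sphere receive a negative, constant-falloff radial force as acceleration, centred on the mesh's relative (not world) location.
; OverlapInnerSphere then destroys the first StaticMeshActor overlapping the inner sphere, indexing the array without a length check.
; Debug text prints during Tick.
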(event `self.ReceiveTick`
  (params (DeltaSeconds :type "Float (single-precision)"))
  (for _array_element (`PrimitiveComponent.GetOverlappingComponents` (`self.OuterSphereComp`))
    (`PrimitiveComponent.AddRadialForce` _array_element (`SceneComponent.RelativeLocation` (`self.MeshComp`)) (`SphereComponent.GetScaledSphereRadius` (`self.OuterSphereComp`)) -2000.0 "RIF_Constant" true))
  (`KismetSystemLibrary.PrintText` "Completed" true true (struct :`G` 0.66 :`B` 1.0 :`A` 1.0) 0.0)
  (`self.OverlapInnerSphere`))

(fn `OverlapInnerSphere`
  (bind _innerspherecomp (`self.InnerSphereComp`))
  (bind _output (`|GetArrayItem` (`PrimitiveComponent.GetOverlappingActors` _innerspherecomp "/Script/Engine.StaticMeshActor")))
  (if (`PrimitiveComponent.IsOverlappingActor` _innerspherecomp _output)
    (`self.K2_DestroyActor` _output)
    (else
      (`KismetSystemLibrary.PrintString` "False" true true (struct :`G` 0.66 :`B` 1.0 :`A` 1.0) 0.0))))

(fn `UserConstructionScript`)